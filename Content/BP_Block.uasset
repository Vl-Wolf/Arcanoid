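; BP_Block is a breakable block that takes two hits from BP_Ball, in a brick-breaker style.
; The first hit swaps the hit component's material, and the next destroys that component and resets the counter.
; Chained, independent random rolls may then spawn a scale, speed or ball bonus at the Box location.
; The scale bonus spawn has no class set, unlike the other two.
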(event EventBeginPlay)

(event Collision|EventActorBeginOverlap
  (params (OtherActor :type Actor%20Object%20Reference)))

(event EventTick
  (params (DeltaSeconds :type Float%20%28single-precision%29)))

(event Collision|EventHit
  (params (MyComp :type Primitive%20Component%20Object%20Reference) (Other :type Actor%20Object%20Reference) (OtherComp :type Primitive%20Component%20Object%20Reference) (bSelfMoved :type Boolean) (HitLocation :type Vector :default "0, 0, 0") (HitNormal :type Vector :default "0, 0, 0") (NormalImpulse :type Vector :default "0, 0, 0") (Hit :type Hit%20Result%20Structure%20%28by%20ref%29))
  (bind _returnvalue (Math|Random|RandomIntegerinRange 0 5))
  (Utilities|Casting|CastToBP_Ball Other)
  (bind _result (Math|Integer|IncrementInt (Variables|Default|GetHintCount))
    (:%20%20
      (if (== _result 1)
        (Rendering|Material|SetMaterial MyComp 0 "/Game/Material_1.Material_1")
        (else
          (Components|DestroyComponent MyComp)
          (Variables|Default|SetHintCount 0)
          (if (== _returnvalue 1)
            (CallFunction|SpawnScaleBonus)
            (elif (== _returnvalue 2)
              (CallFunction|SpawnSpeedBonus)
              (elif (== _returnvalue 3)
                (CallFunction|SpawnBallBonus)))))))))

(fn ConstructionScript)

(fn SpawnScaleBonus
  (Game|SpawnActorfromClass "/Game/BP_BonusScale.BP_BonusScale_C" (Math|Conversions|ToTransform(Vector) (Transformation|GetWorldLocation (Variables|Default|GetBox))) "Undefined" 0 0))

(fn SpawnSpeedBonus
  (Game|SpawnActorfromClass "/Game/BP_BonusSpeed.BP_BonusSpeed_C" (Math|Conversions|ToTransform(Vector) (Transformation|GetWorldLocation (Variables|Default|GetBox))) "Undefined" 0 0))

(fn SpawnBallBonus
  (Game|SpawnActorfromClass "/Game/BP_BonusBall.BP_BonusBall_C" (Math|Conversions|ToTransform(Vector) (Transformation|GetWorldLocation (Variables|Default|GetBox))) "Undefined" 0 0))