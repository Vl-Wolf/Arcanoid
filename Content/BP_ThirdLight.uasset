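; BP_ThirdLight is a light actor whose spotlight blinks a set number of times when play begins.
; The construction script sets the spotlight's initial visibility from IsEnable.
; BeginPlay runs a self-looping DoN that waits Time and toggles visibility on each pass.
; Its limit is twice Flashes, so each flash gets two toggles and the light ends in its starting state.
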(event EventBeginPlay
  (Utilities|FlowControl|DoN (* (Variables|Default|GetFlashes) 2) :!label _label
    (:Exit
      (Utilities|FlowControl|Delay (Variables|Default|GetTime))
      (Rendering|ToggleVisibility (Variables|Default|GetSpotLight) false)
      (goto _label))))

(event Collision|EventActorBeginOverlap
  (params (OtherActor :type Actor%20Object%20Reference)))

(event EventTick
  (params (DeltaSeconds :type Float%20%28single-precision%29)))

(fn ConstructionScript
  (Rendering|SetVisibility (Variables|Default|GetSpotLight) (Variables|Default|GetIsEnable) false))