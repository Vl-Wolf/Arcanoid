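; Player paddle pawn for a ball game, moving sideways and collecting bonuses.
; MoveRight input shifts it by fixed, swept Y offsets per event, and SpaceBar spends a life to spawn a BP_Ball at the capsule.
; Overlapping a BP_Bonus dispatches on its MainBonus name to speed up the last spawned ball, widen the pawn, spawn another ball or add a capped life, then destroys the pickup.
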(event Collision|EventActorBeginOverlap
  (params (OtherActor :type Actor%20Object%20Reference))
  (bind _asbp_bonus (Utilities|Casting|CastToBP_Bonus OtherActor))
  (Variables|Default|SetBP_Bonus _asbp_bonus)
  (if (Utilities|Enum|Equal(Enum) (Variables|/Game/Blueprint/Bonus/BP_Bonus.BP_Bonus_C|GetMainBonus _asbp_bonus) "Speed")
    (CallFunction|SpeedIncrease)
    (Actor|DestroyActor (Variables|Default|GetBP_Bonus))
    (elif (Utilities|Enum|Equal(Enum) (Variables|/Game/Blueprint/Bonus/BP_Bonus.BP_Bonus_C|GetMainBonus _asbp_bonus) "Scale")
      (CallFunction|NewPlayerScale)
      (Actor|DestroyActor (Variables|Default|GetBP_Bonus))
      (elif (Utilities|Enum|Equal(Enum) (Variables|/Game/Blueprint/Bonus/BP_Bonus.BP_Bonus_C|GetMainBonus _asbp_bonus) "Ball")
        (CallFunction|SpawnBall)
        (Actor|DestroyActor (Variables|Default|GetBP_Bonus))
        (elif (Utilities|Enum|Equal(Enum) (Variables|/Game/Blueprint/Bonus/BP_Bonus.BP_Bonus_C|GetMainBonus _asbp_bonus) "Life")
          (CallFunction|LifeIncrease)
          (Actor|DestroyActor (Variables|Default|GetBP_Bonus)))))))

(event Input|AxisEvents|InputAxisMoveRight
  (params (AxisValue :type Float%20%28single-precision%29))
  (if (> AxisValue 0.0)
    (Transformation|AddActorWorldOffset "0,50.000000, 0" true)))

(event Input|AxisEvents|InputAxisMoveRight
  (params (AxisValue :type Float%20%28single-precision%29))
  (if (< AxisValue 0.0)
    (Transformation|AddActorWorldOffset "0,-50.000000, 0" true)))

(event Input|KeyboardEvents|SpaceBar
  (params (Key :type Key%20Structure :default "None"))
  (:Pressed
    (if (> (Variables|Default|GetLives) 0)
      (CallFunction|SpawnBall)
      (bind _result (Math|Integer|DecrementInt (Variables|Default|GetLives))
        (:%20%20
          (Variables|Default|SetLives _result))))))

(fn ConstructionScript)

(fn SpawnBall
  (bind _returnvalue (Game|SpawnActorfromClass "/Game/Blueprint/Player/BP_Ball.BP_Ball_C" (Math|Conversions|ToTransform(Vector) (Transformation|GetWorldLocation (Variables|Default|GetCapsule))) "AlwaysSpawn" 0 0))
  (Variables|Default|SetPlayingBall _returnvalue)
  (if (> (Variables|Default|GetLives) 0)
    _))

(fn NewPlayerScale
  (Transformation|SetActorScale3D (Math|Vector|MakeVector 1.0 (* (Variables|Default|GetPlayerScale) 1.05) 1.0))
  (Variables|Default|SetPlayerScale (* (Variables|Default|GetPlayerScale) 1.05)))

(fn SpeedIncrease
  (bind _playingball (Variables|Default|GetPlayingBall))
  (Variables|/Game/Blueprint/Player/BP_Ball.BP_Ball_C|SetSpeed _playingball (+ (Variables|/Game/Blueprint/Player/BP_Ball.BP_Ball_C|GetSpeed _playingball) 1e+01))
  (return))

(fn LifeIncrease
  (if (<= (Variables|Default|GetLives) 3)
    (Math|Integer|IncrementInt (Variables|Default|GetLives))))