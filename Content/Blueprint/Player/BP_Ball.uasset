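; BP_Ball is a bouncing ball actor that travels at a set speed along a Direction vector.
; Each Tick it moves with a swept world offset, and on a blocking hit plays a sound at the world origin.
; The hit also reflects Direction in X and Y off the surface normal, zeroing Z.
; Overlapping a KillZVolume destroys the ball.
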(event EventBeginPlay)

(event Collision|EventActorBeginOverlap
  (params (OtherActor :type Actor%20Object%20Reference))
  (Utilities|Casting|CastToKillZVolume OtherActor)
  (Actor|DestroyActor))

(event EventTick
  (params (DeltaSeconds :type Float%20%28single-precision%29))
  (bind _sweephitresult (Transformation|AddActorWorldOffset (* (* (Variables|Default|GetDirection) (Variables|Default|GetSpeed)) DeltaSeconds) true))
  (if (.bBlockingHit (Collision|BreakHitResult _sweephitresult))
    (Audio|PlaySoundatLocation "/Game/FX/Sound/Hit.Hit" "0, 0, 0" "0, 0, 0" 1.0 1.0 0.0 0 0 0)
    (Variables|Default|SetDirection (Math|Vector|MakeVector (.x (Math|Vector|GetReflectionVector (Math|Vector|MakeVector (.x (Variables|Default|GetDirection)) (.y (Variables|Default|GetDirection)) 0.0) (Math|Vector|MakeVector (.x (.Normal (Collision|BreakHitResult _sweephitresult))) (.y (.Normal (Collision|BreakHitResult _sweephitresult))) 0.0))) (.y (Math|Vector|GetReflectionVector (Math|Vector|MakeVector (.x (Variables|Default|GetDirection)) (.y (Variables|Default|GetDirection)) 0.0) (Math|Vector|MakeVector (.x (.Normal (Collision|BreakHitResult _sweephitresult))) (.y (.Normal (Collision|BreakHitResult _sweephitresult))) 0.0))) 0.0))))

(fn ConstructionScript)