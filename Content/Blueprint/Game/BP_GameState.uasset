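; Game state Blueprint that tracks the current score and a persistent record score.
; On BeginPlay it restores the record from the "Record" save slot through BP_SaveGame, if that save exists.
; IncrementScore adds a change value to the score.
; NewRecordScore stores the given record and writes it to a freshly created save object in the same slot, without comparing it to the previous record.
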(event EventBeginPlay
  (bind _returnvalue (SaveGame|DoesSaveGameExist "Record"))
  (if _returnvalue
    (bind _returnvalue_2 (SaveGame|LoadGamefromSlot "Record"))
    (bind _asbp_save_game (Utilities|Casting|CastToBP_SaveGame _returnvalue_2))
    (Variables|Default|SetRecordScore (Variables|/Game/Blueprint/Game/BP_SaveGame.BP_SaveGame_C|GetNewRecordScore _asbp_save_game))))

(event EventTick
  (params (DeltaSeconds :type Float%20%28single-precision%29)))

(fn ConstructionScript)

(fn IncrementScore
  (params (ChangeValue :type Integer))
  (Variables|Default|SetScore (+ ChangeValue (Variables|Default|GetScore))))

(fn NewRecordScore
  (params (NewRecord :type Integer))
  (Variables|Default|SetRecordScore NewRecord)
  (bind _returnvalue (SaveGame|CreateSaveGameObject "/Game/Blueprint/Game/BP_SaveGame.BP_SaveGame_C"))
  (bind _output_get (Variables|Default|SetSaveGame _returnvalue))
  (Variables|/Game/Blueprint/Game/BP_SaveGame.BP_SaveGame_C|SetNewRecordScore _output_get (Variables|Default|GetRecordScore))
  (SaveGame|SaveGametoSlot (Variables|Default|GetSaveGame) "Record"))