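; Game mode for a block-destroying game that handles scoring and ending the game.
; DestroyBlock passes positive scores to BP_GameState and updates the record once the score reaches it.
; Only within that record branch does a true result from IncrementScore trigger a win through EndGame_GameMode, which notifies BP_PlayerController and pauses the game.
; The start-game widget creation in the event graph is unconnected and never runs.
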(event EventBeginPlay)

(event EventTick
  (params (DeltaSeconds :type Float%20%28single-precision%29)))

(fn ConstructionScript)

(fn DestroyBlock
  (params (Score :type Integer))
  (if (> Score 0)
    (bind _asbp_game_state (Utilities|Casting|CastToBP_GameState (Game|GetGameState)))
    (bind _biswin (Default|IncrementScore _asbp_game_state Score))
    (bind _asbp_game_state_2 (Utilities|Casting|CastToBP_GameState (Game|GetGameState)))
    (if (>= (Variables|/Game/Blueprint/Game/BP_GameState.BP_GameState_C|GetScore _asbp_game_state_2) (Variables|/Game/Blueprint/Game/BP_GameState.BP_GameState_C|GetRecordScore _asbp_game_state_2))
      (Default|NewRecordScore _asbp_game_state_2 (Variables|/Game/Blueprint/Game/BP_GameState.BP_GameState_C|GetScore _asbp_game_state_2))
      (if _biswin
        (CallFunction|EndGameGameMode true)))))

(fn EndGameGameMode
  (params (bIsWin :type Boolean))
  (bind _asbp_player_controller (Utilities|Casting|CastToBP_PlayerController (Game|GetPlayerController 0)))
  (Default|EndGamePlayerController _asbp_player_controller bIsWin)
  (Game|SetGamePaused true))