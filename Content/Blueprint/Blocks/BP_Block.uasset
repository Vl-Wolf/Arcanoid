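; BP_Block is a hittable block whose Cube material shows its health and which can drop a bonus.
; On BeginPlay it picks the material from BPHealthComponent's Health.
; Each Hit passes 1 to ChangeHealth, then, if the component is still valid, applies a hit material based on the new Health.
; SpawnBonus spawns BP_Bonus at the Box location when a random roll exceeds DropChance, but nothing here calls it.
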(event EventBeginPlay
  (Rendering|Material|SetMaterial (Variables|Default|GetCube) 0 (Utilities|Select :Index (Variables|/Game/Blueprint/ActorComponent/BP_HealthComponent.BP_HealthComponent_C|GetHealth (Variables|Default|GetBP_HealthComponent)) :Option%200 "/Game/FX/Material/BlockMaterial/BlockMaterial_1.BlockMaterial_1" :Option%201 "/Game/FX/Material/BlockMaterial/BlockMaterial_2.BlockMaterial_2" :Option%202 "/Game/FX/Material/BlockMaterial/BlockMaterial_3.BlockMaterial_3")))

(event Collision|EventHit
  (params (MyComp :type Primitive%20Component%20Object%20Reference) (Other :type Actor%20Object%20Reference) (OtherComp :type Primitive%20Component%20Object%20Reference) (bSelfMoved :type Boolean) (HitLocation :type Vector :default "0, 0, 0") (HitNormal :type Vector :default "0, 0, 0") (NormalImpulse :type Vector :default "0, 0, 0") (Hit :type Hit%20Result%20Structure%20%28by%20ref%29))
  (bind _bp_healthcomponent (Variables|Default|GetBP_HealthComponent))
  (bind _cube (Variables|Default|GetCube))
  (Default|ChangeHealth _bp_healthcomponent 1)
  (Utilities|IsValid _bp_healthcomponent
    (:Is%20Valid
      (if (== (Variables|/Game/Blueprint/ActorComponent/BP_HealthComponent.BP_HealthComponent_C|GetHealth _bp_healthcomponent) 1)
        (Rendering|Material|SetMaterial _cube 0 "/Game/FX/Material/HitMaterial/HitMaterial_0255.HitMaterial_0255")
        (else
          (Rendering|Material|SetMaterial _cube 0 "/Game/FX/Material/HitMaterial/HitMaterial_075.HitMaterial_075"))))))

(fn ConstructionScript)

(fn SpawnBonus
  (if (> (Math|Random|RandomFloat) (Variables|Default|GetDropChance))
    (Game|SpawnActorfromClass "/Game/Blueprint/Bonus/BP_Bonus.BP_Bonus_C" (Math|Conversions|ToTransform(Vector) (Transformation|GetWorldLocation (Variables|Default|GetBox))) "Undefined" 0 0)))