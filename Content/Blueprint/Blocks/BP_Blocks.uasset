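; BP_Blocks is a block layout actor that builds a flat grid of child actors in its construction script.
; Nested loops over X and Y add a scaled-up child actor component only where both indices are odd, leaving every other cell empty.
; Each position is the index times Padding, so neighbors sit two Padding units apart.
; BeginPlay is empty, so the asset has no runtime logic of its own.
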(event EventBeginPlay)

(fn ConstructionScript
  (for _index (range 1 (Variables|Default|GetX))
    (if (!= (Math|Integer|%(Integer) _index 2) 0)
      (for _index_2 (range 1 (Variables|Default|GetY))
        (if (!= (Math|Integer|%(Integer) _index_2 2) 0)
          (AddComponent|AddChildActorComponent false (Math|Transform|MakeTransform (Math|Vector|MakeVector (Math|Conversions|ToFloat(Integer) (* _index (* (Math|Integer|%(Integer) _index 2) (Variables|Default|GetPadding)))) (Math|Conversions|ToFloat(Integer) (* _index_2 (* (Math|Integer|%(Integer) _index_2 2) (Variables|Default|GetPadding)))) 0.0) "0, 0, 0" "1.500000,1.500000,1.500000")))))))