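; BP_Bonus is a moving pickup actor that represents one of four randomly chosen bonus types: speed, scale, ball or life.
; On BeginPlay it rolls a random index, stores the matching entry of BonusName in MainBonus and applies that type's material to its cube.
; Each Tick it moves along Direction at Speed, scaled by delta time, using a swept offset.
; The bonus effect itself is not applied here.
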(event EventBeginPlay
  (bind _output_get (Variables|Default|SetRnd (Math|Random|RandomIntegerinRange 0 3)))
  (Variables|Default|SetMainBonus (Utilities|Array|Get(acopy) (Variables|Default|GetBonusName) _output_get))
  (Rendering|Material|SetMaterial (Variables|Default|GetCube) 0 (Utilities|Select :Index _output_get :Option%200 "/Game/FX/Material/BonusMaterial/SpeedMaterial.SpeedMaterial" :Option%201 "/Game/FX/Material/BonusMaterial/ScaleMaterial.ScaleMaterial" :Option%202 "/Game/FX/Material/BonusMaterial/BallMaterial.BallMaterial" :Option%203 "/Game/FX/Material/BonusMaterial/LifeMaterial.LifeMaterial")))

(event EventTick
  (params (DeltaSeconds :type Float%20%28single-precision%29))
  (Transformation|AddActorWorldOffset (* (* (Variables|Default|GetDirection) (Variables|Default|GetSpeed)) DeltaSeconds) true))

(fn ConstructionScript)